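; Base player ship pawn that routes flight input to BPShipMovementComponent, which Tick drives through movement and braking.
; A toggle switches between default mode, where mouse steers and move inputs translate the ship, and alt mode, where mouse orbits the spring arm and move inputs turn.
; Alt mode moves continuously, stepping thrust by buttons and reversing at zero.
; Default mode locks the camera to the ship and zeroes thrust when nearly stopped.
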(event EventTick
  (params (DeltaSeconds :type Float%20%28single-precision%29))
  (if (Variables|Movement|GetIsAltController)
    (Default|AddForwardMovement (Variables|Default|GetBP_ShipMovementComponent) (select (Variables|Movement|GetIsReverse) -1.0 1.0))
    (else
      (CallFunction|ResetSpringArmRotation)))
  (Default|Move (Variables|Default|GetBP_ShipMovementComponent))
  (Default|Braking (Variables|Default|GetBP_ShipMovementComponent))
  (if (not (Variables|Movement|GetIsAltController))
    (if (Utilities|Operators|EqualEqual :A (Variables|/Game/Game/Blueprints/BP_ShipMovementComponent.BP_ShipMovementComponent_C|GetVelocity (Variables|Default|GetBP_ShipMovementComponent)) :ErrorTolerance 8.0)
      (Variables|/Game/Game/Blueprints/BP_ShipMovementComponent.BP_ShipMovementComponent_C|SetThrasholdIndex (Variables|Default|GetBP_ShipMovementComponent) 0))))

(event Input|ActionEvents|InputActionAltControllerAddSpeed
  (params (Key :type Key%20Structure :default "None"))
  (:Pressed
    (if (Variables|Movement|GetIsAltController)
      (CallFunction|SetReverse false)
      (Default|IncForwardThrust (Variables|Default|GetBP_ShipMovementComponent)))))

(event Input|ActionEvents|InputActionAltControllerDecSpeed
  (params (Key :type Key%20Structure :default "None"))
  (:Pressed
    (if (Variables|Movement|GetIsAltController)
      (if (not (Variables|Movement|GetIsReverse))
        (if (== 0 (Variables|/Game/Game/Blueprints/BP_ShipMovementComponent.BP_ShipMovementComponent_C|GetThrasholdIndex (Variables|Default|GetBP_ShipMovementComponent)))
          (CallFunction|SetReverse true)
          (else
            (Default|DecForwardThrust (Variables|Default|GetBP_ShipMovementComponent))))))))

(event Input|ActionEvents|InputActionSwitchController
  (params (Key :type Key%20Structure :default "None"))
  (:Pressed
    (Variables|Movement|SetIsAltController (not (Variables|Movement|GetIsAltController)))
    (CallFunction|SetReverse false)))

(event Input|AxisEvents|InputAxisLookUp/DownMouse
  (params (AxisValue :type Float%20%28single-precision%29))
  ;[1 1 1] Camera
  (if (Variables|Movement|GetIsAltController)
    (Transformation|AddLocalRotation (Variables|Default|GetSpringArm) (Math|Rotator|MakeRotator 0.0 AxisValue 0.0) false false)
    (else
      (Default|AddPitchRotation (Variables|Default|GetBP_ShipMovementComponent) AxisValue))))

(event Input|AxisEvents|InputAxisTurnRight/LeftMouse
  (params (AxisValue :type Float%20%28single-precision%29))
  ;[1 1 1] Camera
  (if (Variables|Movement|GetIsAltController)
    (Transformation|AddLocalRotation (Variables|Default|GetSpringArm) (Math|Rotator|MakeRotator 0.0 0.0 AxisValue) false false)
    (else
      (Default|AddYawRotation (Variables|Default|GetBP_ShipMovementComponent) AxisValue))))

(event Input|AxisEvents|InputAxisRoll
  (params (AxisValue :type Float%20%28single-precision%29))
  ;[1 1 1] Camera
  (Default|AddRollRotation (Variables|Default|GetBP_ShipMovementComponent) AxisValue))

(event Input|AxisEvents|InputAxisMoveRight/Left
  (params (AxisValue :type Float%20%28single-precision%29))
  (if (Variables|Movement|GetIsAltController)
    (Default|AddYawRotation (Variables|Default|GetBP_ShipMovementComponent) AxisValue)
    (else
      (Default|AddRightMovement (Variables|Default|GetBP_ShipMovementComponent) AxisValue))))

(event Input|AxisEvents|InputAxisMoveUp/Down
  (params (AxisValue :type Float%20%28single-precision%29))
  (if (Variables|Movement|GetIsAltController)
    (Default|AddPitchRotation (Variables|Default|GetBP_ShipMovementComponent) AxisValue)
    (else
      (Default|AddUpMovement (Variables|Default|GetBP_ShipMovementComponent) AxisValue))))

(event Input|AxisEvents|InputAxisMoveForward/Backward
  (params (AxisValue :type Float%20%28single-precision%29))
  (if (not (Math|Float|NearlyEqual(Float) AxisValue 0.0 0.001))
    (if (not (Variables|Movement|GetIsAltController))
      (if (== (Variables|/Game/Game/Blueprints/BP_ShipMovementComponent.BP_ShipMovementComponent_C|GetThrasholdIndex (Variables|Default|GetBP_ShipMovementComponent)) 0)
        (Default|IncForwardThrust (Variables|Default|GetBP_ShipMovementComponent)))
      (Default|AddForwardMovement (Variables|Default|GetBP_ShipMovementComponent) AxisValue))))

(event Input|AxisEvents|InputAxisSpeedUp/DownMouse
  (params (AxisValue :type Float%20%28single-precision%29))
  (Default|AddForwardThrust (Variables|Default|GetBP_ShipMovementComponent) (Math|Float|Truncate AxisValue)))

(fn ConstructionScript)

(fn ResetSpringArmRotation
  (Transformation|SetWorldRotation (Variables|Default|GetSpringArm) (Transformation|GetWorldRotation (Variables|Default|GetShipRoot)) false false))

(fn DrawDebugAxis
  (params (axis :type Vector) (NewParam :type Linear%20Color%20Structure))
  (bind _returnvalue (Transformation|GetActorLocation))
  (Rendering|Debug|DrawDebugLine _returnvalue (+ _returnvalue (* axis 3e+02)) NewParam 0.0 0.0))

(fn SetReverse
  (params (NewReverse :type Boolean))
  (Variables|Movement|SetIsReverse NewReverse))