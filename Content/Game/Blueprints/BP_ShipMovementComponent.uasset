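; Movement component that flies its owning ship with stepped forward throttle, side thrusters and three-axis rotation.
; Directional inputs accumulate thrust along the actor's axes into Velocity, which Move applies as a swept world offset and Braking eases toward zero.
; Forward thrust scales with the square of the clamped throttle index and boosts tenfold during acceleration, while reverse uses side thrust.
; Yaw, pitch and roll rotate the owner directly, without inertia.
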(event EventBeginPlay)

(fn AddForwardThrust
  (params (AxisValue :type Integer))
  (Variables|Default|SetThrasholdIndex (Math|Integer|Clamp(Integer) (+ AxisValue (Variables|Default|GetThrasholdIndex)) 0 (Variables|ThrasholdRange|GetThrasholdIndexMax))))

(fn IncForwardThrust
  (Variables|Default|SetThrasholdIndex (Math|Integer|Clamp(Integer) (+ (Variables|Default|GetThrasholdIndex) 1) (Variables|ThrasholdRange|GetThrasholdIndexMin) (Variables|ThrasholdRange|GetThrasholdIndexMax))))

(fn DecForwardThrust
  (Variables|Default|SetThrasholdIndex (Math|Integer|Clamp(Integer) (- (Variables|Default|GetThrasholdIndex) 1) (Variables|ThrasholdRange|GetThrasholdIndexMin) (Variables|ThrasholdRange|GetThrasholdIndexMax))))

(fn AddYawRotation
  (params (AxisValue :type Float%20%28double-precision%29))
  (Transformation|AddActorLocalRotation (Components|GetOwner) (Math|Rotator|MakeRotator 0.0 0.0 (* AxisValue (* (Utilities|Time|GetWorldDeltaSeconds) (Variables|Thrust|GetRotationPower)))) true false))

(fn AddPitchRotation
  (params (AxisValue :type Float%20%28double-precision%29))
  (Transformation|AddActorLocalRotation (Components|GetOwner) (Math|Rotator|MakeRotator 0.0 (* AxisValue (* (Utilities|Time|GetWorldDeltaSeconds) (Variables|Thrust|GetRotationPower))) 0.0) true false))

(fn AddRollRotation
  (params (AxisValue :type Float%20%28double-precision%29))
  (Transformation|AddActorLocalRotation (Components|GetOwner) (Math|Rotator|MakeRotator (* AxisValue (* (Utilities|Time|GetWorldDeltaSeconds) (Variables|Thrust|GetRotationPower))) 0.0 0.0) true false))

(fn Braking
  (Variables|Default|SetVelocity (Math|Interpolation|VInterpTo (Variables|Default|GetVelocity) "0, 0, 0" (Utilities|Time|GetWorldDeltaSeconds) (Variables|Thrust|GetBrakingFactor))))

(fn Move
  (Transformation|AddActorWorldOffset (Components|GetOwner) (Variables|Default|GetVelocity) true))

(fn GetForwardThrust
  (bind _thrasholdindex (Variables|Default|GetThrasholdIndex))
  (return (* (* (Variables|Thrust|GetThrust) (* _thrasholdindex _thrasholdindex)) (select (Variables|Default|GetIsAcceleration) 10 1))))

(fn GetSideThrust
  (return (Variables|Thrust|GetSideThrust)))

(fn AddForwardMovement
  (params (AxisValue :type Float%20%28double-precision%29))
  (Variables|Default|SetVelocity (+ (Variables|Default|GetVelocity) (* (* (* AxisValue (select (< AxisValue 0.0) (CallFunction|GetSideThrust) (CallFunction|GetForwardThrust))) (Utilities|Time|GetWorldDeltaSeconds)) (Transformation|GetActorForwardVector (Components|GetOwner))))))

(fn AddRightMovement
  (params (AxisValue :type Float%20%28double-precision%29))
  (Variables|Default|SetVelocity (+ (Variables|Default|GetVelocity) (* (* (* AxisValue (CallFunction|GetSideThrust)) (Utilities|Time|GetWorldDeltaSeconds)) (Transformation|GetActorRightVector (Components|GetOwner))))))

(fn AddUpMovement
  (params (AxisValue :type Float%20%28double-precision%29))
  (Variables|Default|SetVelocity (+ (Variables|Default|GetVelocity) (* (* (* AxisValue (CallFunction|GetSideThrust)) (Utilities|Time|GetWorldDeltaSeconds)) (Transformation|GetActorUpVector (Components|GetOwner))))))