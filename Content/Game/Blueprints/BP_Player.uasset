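; BP_Player is a player Character that flies freely with six degrees of freedom and adjustable speed.
; Movement axes push along the actor's own forward, right and up vectors, while look and roll axes rotate the actor locally, bypassing controller rotation.
; A speed axis changes MaxFlySpeed, scaled by delta time and SpeedVelocity.
; Tick restores DefaultSpeed whenever the last update velocity is near zero.
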(event EventBeginPlay)

(event Collision|EventActorBeginOverlap
  (params (OtherActor :type Actor%20Object%20Reference)))

(event EventTick
  (params (DeltaSeconds :type Float%20%28single-precision%29))
  (if (Utilities|Operators|EqualEqual :A (Pawn|Components|CharacterMovement|GetLastUpdateVelocity (Variables|Character|GetCharacterMovement)) :ErrorTolerance 2e+01)
    (Variables|/Script/Engine.CharacterMovementComponent|SetMaxFlySpeed (Variables|Character|GetCharacterMovement) (Variables|Default|GetDefaultSpeed))))

(event Input|AxisEvents|InputAxisMoveForward/Backward
  (params (AxisValue :type Float%20%28single-precision%29))
  ;[0.15 0.15 0.15] Move
  (Pawn|Input|AddMovementInput (Transformation|GetActorForwardVector) AxisValue false))

(event Input|AxisEvents|InputAxisMoveRight/Left
  (params (AxisValue :type Float%20%28single-precision%29))
  ;[0.15 0.15 0.15] Move
  (Pawn|Input|AddMovementInput (Transformation|GetActorRightVector) AxisValue false))

(event Input|AxisEvents|InputAxisTurnRight/LeftMouse
  (params (AxisValue :type Float%20%28single-precision%29))
  ;[0.25 0.25 0.25] Camera
  (Transformation|AddActorLocalRotation (Math|Rotator|MakeRotator 0.0 0.0 AxisValue) false false))

(event Input|AxisEvents|InputAxisLookUp/DownMouse
  (params (AxisValue :type Float%20%28single-precision%29))
  ;[0.25 0.25 0.25] Camera
  (Transformation|AddActorLocalRotation (Math|Rotator|MakeRotator 0.0 AxisValue 0.0) false false))

(event Input|AxisEvents|InputAxisSpeedUp/DownMouse
  (params (AxisValue :type Float%20%28single-precision%29))
  (bind _charactermovement (Variables|Character|GetCharacterMovement))
  ;[0.35 0.35 0.35] Speed
  (Variables|/Script/Engine.CharacterMovementComponent|SetMaxFlySpeed _charactermovement (+ (* (* AxisValue (Utilities|Time|GetWorldDeltaSeconds)) (Variables|Default|GetSpeedVelocity)) (Variables|/Script/Engine.CharacterMovementComponent|GetMaxFlySpeed _charactermovement))))

(event Input|AxisEvents|InputAxisMoveUp/Down
  (params (AxisValue :type Float%20%28single-precision%29))
  ;[0.15 0.15 0.15] Move
  (Pawn|Input|AddMovementInput (Transformation|GetActorUpVector) AxisValue false))

(event Input|AxisEvents|InputAxisRoll
  (params (AxisValue :type Float%20%28single-precision%29))
  ;[0.25 0.25 0.25] Camera
  (Transformation|AddActorLocalRotation (Math|Rotator|MakeRotator AxisValue 0.0 0.0) false false))

(fn ConstructionScript)